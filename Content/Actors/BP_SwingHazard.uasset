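; Swinging wrecking-ball hazard that pushes its WreckingBall with repeated physics impulses, starting clockwise on BeginPlay.
; Looping timers, set to the frame delta cached in Tick, call swing functions that apply ImpulseVector or its negation and print debug text.
; Each function adds to a shared TimeCounter and starts the opposite timer past a threshold.
; The counter is never reset, and switching never clears the other direction's timer.
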(event `self.ReceiveBeginPlay`
  (`self.StartSwingingClockwise`))

(event `StartSwingingClockwise`
  (if (not (not (`KismetSystemLibrary.K2_IsValidTimerHandle` (stale _returnvalue))))
    (`KismetSystemLibrary.K2_ClearAndInvalidateTimerHandle` (stale _returnvalue)))
  (bind _returnvalue (`KismetSystemLibrary.K2_SetTimer` null "SwingClockwise" (`self.DeltaTime`) true)))

(event `StartSwingingAnticlockwise`
  (if (not (not (`KismetSystemLibrary.K2_IsValidTimerHandle` (stale _returnvalue))))
    (`KismetSystemLibrary.K2_ClearAndInvalidateTimerHandle` (stale _returnvalue)))
  (bind _returnvalue (`KismetSystemLibrary.K2_SetTimer` null "SwingAnticlockwise" (`self.DeltaTime`) true)))

(event `self.ReceiveTick`
  (params (DeltaSeconds :type "Float (single-precision)"))
  (set `self.DeltaTime` DeltaSeconds))

(fn `SwingAnticlockwise`
  (bind _output_get (set `self.OppositeImpluseVector` (`KismetMathLibrary.MakeVector` (* (.x (`self.ImpulseVector`)) -1.0) (* (.y (`self.ImpulseVector`)) -1.0) (* (.z (`self.ImpulseVector`)) -1.0))))
  (`KismetSystemLibrary.PrintString` "Swing Anticlockwise")
  (`PrimitiveComponent.AddImpulse` (`self.WreckingBall`) _output_get "None" false)
  (bind _output_get_2 (set `self.TimeCounter` (+ (`self.DeltaTime`) (`self.TimeCounter`))))
  (if (>= _output_get_2 (`self.TotalTimeForDirectionChange`))
    (`self.StartSwingingClockwise`)))

(fn `SwingClockwise`
  (`KismetSystemLibrary.PrintString` "Swing Clockwise" true true (struct :`G` 0.66 :`B` 1.0 :`A` 1.0) 0.1)
  (`PrimitiveComponent.AddImpulse` (`self.WreckingBall`) (`self.ImpulseVector`) "None" false)
  (bind _output_get (set `self.TimeCounter` (+ (`self.DeltaTime`) (`self.TimeCounter`))))
  (if (>= _output_get (`self.TotalTimeForDirectionChange`))
    (`self.StartSwingingAntiClockwise`)))

(fn `UserConstructionScript`)