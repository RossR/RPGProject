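; Player controller for an RPG project, holding sprint and jump logic for the controlled Character, none of which is wired to an event.
; Two sprint chains switch CharacterMovement walk speed, minimum analog speed and acceleration between fast and normal values.
; Two further chains call Jump and StopJumping on the pawn.
; BeginPlay, Tick and the construction script are empty, so the controller runs no logic of its own.
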(event `InputAction|Sprint`
  (params (Key :type "Key Structure"))
  ;[1 0 0.02448] Sprint Action
)

(event `InputAction|Jump`
  (params (Key :type "Key Structure")))

(fn `UserConstructionScript`)