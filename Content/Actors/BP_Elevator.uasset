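; Elevator actor meant to shuttle between its starting location and an offset end point computed in the construction script.
; A looping timer starts after a delay and calls ElevatorUp, which steps the actor upward in fixed increments until it matches the end point.
; ToggleDirection then clears the timers and schedules up or down travel by comparing location to the start.
; ElevatorDown is empty, so the descent is unimplemented.
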(event `self.ReceiveBeginPlay`
  (bind _returnvalue (`KismetSystemLibrary.K2_SetTimer` null "ElevatorUp" 0.1 true 5.0))
  (`KismetSystemLibrary.PrintString` "timer started"))

(event `ToggleDirection`
  (`KismetSystemLibrary.K2_ClearAndInvalidateTimerHandle` (stale `self.ReceiveBeginPlay` _returnvalue))
  (`KismetSystemLibrary.K2_ClearAndInvalidateTimerHandle` (stale _returnvalue))
  (`KismetSystemLibrary.K2_ClearAndInvalidateTimerHandle` (stale _returnvalue_2))
  (if (== (`SceneComponent.K2_GetComponentLocation` (`self.StaticMeshComponent`)) (`self.StartingTransform`))
    (bind _returnvalue (`KismetSystemLibrary.K2_SetTimer` null "ElevatorUp" (`GameplayStatics.GetWorldDeltaSeconds`) true 5.0))
    (else
      (bind _returnvalue_2 (`KismetSystemLibrary.K2_SetTimer` null "ElevatorDown" (`GameplayStatics.GetWorldDeltaSeconds`) true 5.0)))))

(fn `ElevatorDown`)

(fn `ElevatorUp`
  (`KismetSystemLibrary.PrintString` "ElevatorUp")
  (if (== (`SceneComponent.K2_GetComponentLocation` (`self.StaticMeshComponent`)) (`self.EndTransform`))
    (`self.ToggleDirection`)
    (else
      (`self.K2_SetActorTransform` (`KismetMathLibrary.Conv_VectorToTransform` (+ (`SceneComponent.K2_GetComponentLocation` (`self.StaticMeshComponent`)) (/ (0.0 0.0 10.0) 1.0)))))))

(fn `UserConstructionScript`
  (bind _output_get (set `self.StartingTransform` (`SceneComponent.K2_GetComponentLocation` (`self.StaticMeshComponent`))))
  (set `self.EndTransform` (+ _output_get (`self.TargetTransform`))))