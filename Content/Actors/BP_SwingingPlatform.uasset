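; BP_SwingingPlatform is a physics platform built to swing back and forth, though its start logic is disconnected, leaving BeginPlay empty.
; Looping timers, timed by DeltaSeconds, call SwingClockwise or SwingAnticlockwise to apply opposing impulses.
; Passing the roll limit sets a small linear velocity along the current impulse, then starts the opposite timer.
; The start events clear the other timer only when it is inactive, so active timers keep running.
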(event `self.ReceiveBeginPlay`)

(event `StartSwingingClockwise`
  (if (not (`KismetSystemLibrary.K2_IsTimerActiveHandle` (stale `StartSwingingAnticlockwise` _returnvalue)))
    (`KismetSystemLibrary.K2_ClearAndInvalidateTimerHandle` (stale `StartSwingingAnticlockwise` _returnvalue)))
  (bind _returnvalue (`KismetSystemLibrary.K2_SetTimer` null "SwingClockwise" (`self.Delta Seconds`) true)))

(event `StartSwingingAnticlockwise`
  (if (not (`KismetSystemLibrary.K2_IsTimerActiveHandle` (stale `StartSwingingClockwise` _returnvalue)))
    (`KismetSystemLibrary.K2_ClearAndInvalidateTimerHandle` (stale `StartSwingingClockwise` _returnvalue)))
  (bind _returnvalue (`KismetSystemLibrary.K2_SetTimer` null "SwingAnticlockwise" (`self.Delta Seconds`) true)))

(event `self.ReceiveTick`
  (params (DeltaSeconds :type "Float (single-precision)"))
  (set `self.Delta Seconds` DeltaSeconds))

(fn `SwingAnticlockwise`
  (bind _impulse_vector (`self.Impulse Vector`))
  (bind _relativerotation_roll (`KismetMathLibrary.BreakRotator` (`SceneComponent.RelativeRotation` (`self.SwingingPlatform`))))
  (`PrimitiveComponent.AddImpulse` (`self.SwingingPlatform`) _impulse_vector "None" false)
  (`KismetSystemLibrary.PrintString` "Anticlockwise" true true (struct :`G` 0.66 :`B` 1.0 :`A` 1.0) 0.1)
  (if (<= _relativerotation_roll (* (`self.DirectionChangeAngle`) -1.0))
    (`/Engine/EditorBlueprintResources/StandardMacros.DoOnce` false :!label _label
      (:`Completed`
        (`PrimitiveComponent.SetAllPhysicsLinearVelocity` (`self.SwingingPlatform`) (* _impulse_vector 0.1) false)
        (`self.StartSwingingClockwise`)))
    (else
      (goto _label :!via `Reset`))))

(fn `SwingClockwise`
  (bind _relativerotation_roll (`KismetMathLibrary.BreakRotator` (`SceneComponent.RelativeRotation` (`self.SwingingPlatform`))))
  (bind _returnvalue (`KismetMathLibrary.MakeVector` (* (.x (`self.Impulse Vector`)) -1.0) (* (.y (`self.Impulse Vector`)) -1.0) (* (.z (`self.Impulse Vector`)) -1.0)))
  (`PrimitiveComponent.AddImpulse` (`self.SwingingPlatform`) _returnvalue "None" false)
  (`KismetSystemLibrary.PrintString` "Clockwise" true true (struct :`G` 0.66 :`B` 1.0 :`A` 1.0) 0.1)
  (if (>= _relativerotation_roll (`self.DirectionChangeAngle`))
    (`/Engine/EditorBlueprintResources/StandardMacros.DoOnce` false :!label _label
      (:`Completed`
        (`PrimitiveComponent.SetAllPhysicsLinearVelocity` (`self.SwingingPlatform`) (* _returnvalue 0.1) false)
        (`self.StartSwingingAnticlockwise`)))
    (else
      (goto _label :!via `Reset`))))

(fn `UserConstructionScript`)