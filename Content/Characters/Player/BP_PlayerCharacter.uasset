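; Player character Blueprint that tags itself as the player and handles a toggleable spotlight and target-focus input.
; The L key flips the SpotLight component's visibility on and off.
; The FocusTarget action flips a LookAt flag, which nothing in this file reads.
; BeginPlay replaces the tags of player character 0 with a single Player tag.
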(event `Key|L`
  (params (Key :type "Key Structure"))
  (bind _spotlight (`self.SpotLight`))
  (:`Pressed`
    (`/Engine/EditorBlueprintResources/StandardMacros.FlipFlop`
      (:`A`
        (`SceneComponent.SetVisibility` _spotlight true false))
      (:`B`
        (`SceneComponent.SetVisibility` _spotlight false false)))))

(event `self.ReceiveBeginPlay`
  (set `Actor.Tags` (`|MakeArray` "Player" :!type "Name") (`GameplayStatics.GetPlayerCharacter` 0)))

(event `InputAction|FocusTarget`
  (params (Key :type "Key Structure"))
  ;[1 1 1] Toggle LookAt
  (:`Pressed`
    (`/Engine/EditorBlueprintResources/StandardMacros.FlipFlop`
      (:`A`
        (set `self.LookAt` true))
      (:`B`
        (set `self.LookAt` false)))))

(fn `UserConstructionScript`)