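; Player controller for the RPG player character that creates the HUD and manages the character details and inventory menus.
; BeginPlay caches the controlled pawn and adds the HUD widget to the viewport.
; B and I each use a FlipFlop to show or hide their drag window, switching input mode, cursor and the shared IsInMenu flag.
; Tick copies the inventory UI's item and widget maps onto the controller every frame.
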(event `self.ReceiveBeginPlay`
  (`|ExecutionSequence`
    (:`then_0`
      (bind _asbp_rpgproject_player_character (cast `/Game/Characters/Player/BP_RPGProjectPlayerCharacter` (`self.K2_GetPawn` self)))
      (set `self.PlayerCharacter` _asbp_rpgproject_player_character))
    (:`then_1`
      (bind _returnvalue (`|CreateWidget` "/Game/Widgets/WBP_PlayerHUD.WBP_PlayerHUD_C" self))
      (bind _output_get (set `self.PlayerHUDWidget` _returnvalue))
      (`UserWidget.AddToViewport` _output_get 0))))

(event `self.ReceiveTick`
  (params (DeltaSeconds :type "Float (single-precision)"))
  (bind _wbp_inventoryui (`/Game/Widgets/WBP_PlayerHUD.WBP_InventoryUI` (`self.PlayerHUDWidget`)))
  (set `self.InventoryItemMap` (`/Game/Widgets/WBP_InventoryUI.InventoryItemMap` _wbp_inventoryui))
  (set `self.ItemWidgetMap` (`/Game/Widgets/WBP_InventoryUI.ItemWidgetMap` _wbp_inventoryui)))

(event `Key|B`
  (params (Key :type "Key Structure"))
  (bind _playerhudwidget (`self.PlayerHUDWidget`))
  (bind _wbp_dragwindow_characterdetails (`/Game/Widgets/WBP_PlayerHUD.WBP_DragWindow_CharacterDetails` _playerhudwidget))
  (bind _wbp_characterdetails (`/Game/Widgets/WBP_PlayerHUD.WBP_CharacterDetails` _playerhudwidget))
  ;[1 1 1] Open/Close Character Details Menu
  (:`Pressed`
    (`/Engine/EditorBlueprintResources/StandardMacros.IsValid` _wbp_characterdetails
      (:`Is Valid`
        (`/Engine/EditorBlueprintResources/StandardMacros.FlipFlop`
          (:`A`
            (`Widget.SetVisibility` _wbp_dragwindow_characterdetails "Visible")
            (set `self.bIsInMenu` true)
            (`WidgetBlueprintLibrary.SetInputMode_GameAndUIEx` self _wbp_characterdetails)
            (set `self.bShowMouseCursor` true))
          (:`B`
            (`Widget.SetVisibility` _wbp_dragwindow_characterdetails "Hidden")
            (set `self.bIsInMenu` false)
            (set `self.bShowMouseCursor` false)
            (`WidgetBlueprintLibrary.SetInputMode_GameOnly` self))))
      (:`Is Not Valid`
        (`KismetSystemLibrary.PrintString` "Hello")))))

(event `Key|I`
  (params (Key :type "Key Structure"))
  (bind _playerhudwidget (`self.PlayerHUDWidget`))
  (bind _wbp_inventoryui (`/Game/Widgets/WBP_PlayerHUD.WBP_InventoryUI` _playerhudwidget))
  (bind _wbp_dragwindow_inventoryui (`/Game/Widgets/WBP_PlayerHUD.WBP_DragWindow_InventoryUI` _playerhudwidget))
  ;[1 1 1] Open/Close Inventory Menu
  (:`Pressed`
    (`/Engine/EditorBlueprintResources/StandardMacros.IsValid` _wbp_inventoryui
      (:`Is Valid`
        (`/Engine/EditorBlueprintResources/StandardMacros.FlipFlop`
          (:`A`
            (`Widget.SetVisibility` _wbp_dragwindow_inventoryui "Visible")
            (set `self.bIsInMenu` true)
            (`WidgetBlueprintLibrary.SetInputMode_GameAndUIEx` self _wbp_inventoryui)
            (set `self.bShowMouseCursor` true))
          (:`B`
            (`Widget.SetVisibility` _wbp_dragwindow_inventoryui "Hidden")
            (set `self.bIsInMenu` false)
            (set `self.bShowMouseCursor` false)
            (`WidgetBlueprintLibrary.SetInputMode_GameOnly` self))))
      (:`Is Not Valid`
        (`KismetSystemLibrary.PrintString` "Hello")))))

(fn `UserConstructionScript`)