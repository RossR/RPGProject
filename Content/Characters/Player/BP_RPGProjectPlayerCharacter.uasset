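; Player character for the RPG, handling weapons, combat input, dodge rolls, doors and item pickup.
; Number keys swap the ChildActor weapon, socketed by combat state, and its type selects the dodge montage section.
; Inputs set attack and action states, with montages locking out conflicting actions and a notify opening doors.
; Tick runs a head-socket pickup trace feeding the inventory component and interpolates foot-trace IK offsets for feet and hips.
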(event `Key|One`
  (params (Key :type "Key Structure"))
  ;[1 1 1] Change Weapon
  (:`Pressed`
    (`ChildActorComponent.SetChildActorClass` (`self.EquippedWeapon`) "/Game/Actors/Items/Weapon/BP_Sword.BP_Sword_C")
    (bind _asweapon_base (cast `WeaponBase` (`ChildActorComponent.ChildActor` (`self.EquippedWeapon`)) :!label _label))
    (bind _returnvalue (`self.GetPlayerCombatState`))
    (switch `EPlayerCombatState` _returnvalue
      (:`PCS_AtEase`
        (`self.AttachWeaponToSocket` (`WeaponBase.SheathSocket` _asweapon_base)))
      (:`PCS_CombatReady`
        (`self.AttachWeaponToSocket` (`WeaponBase.EquippedSocket` _asweapon_base))))))

(event `Key|Two`
  (params (Key :type "Key Structure"))
  ;[1 1 1] Change Weapon
  (:`Pressed`
    (`ChildActorComponent.SetChildActorClass` (`self.EquippedWeapon`) "/Game/Actors/Items/Weapon/BP_Unarmed.BP_Unarmed_C")
    (goto _label)))

(event `Key|Three`
  (params (Key :type "Key Structure"))
  ;[1 1 1] Change Weapon
  (:`Pressed`
    (`ChildActorComponent.SetChildActorClass` (`self.EquippedWeapon`) "/Game/Actors/Items/Weapon/BP_2HandSpear.BP_2HandSpear_C")
    (goto _label)))

(event `InputAction|ReadyWeapon`
  (params (Key :type "Key Structure"))
  ;[1 1 1] Combat State Flip Flop
  (:`Pressed`
    (if (`|EnumEquality` (`self.PlayerActionState`) "PAS_Idle")
      (`/Engine/EditorBlueprintResources/StandardMacros.FlipFlop`
        (:`A`
          (`self.SetPlayerCombatState` "PCS_CombatReady"))
        (:`B`
          (`self.SetPlayerCombatState` "PCS_AtEase"))))))

(event `InputAction|LightAttack`
  (params (Key :type "Key Structure"))
  ;[1 1 1] IsAttacking - True/False
  (:`Pressed`
    (bind _returnvalue (`self.IsCharacterExhausted`))
    (if (and (and (not _returnvalue) (`|EnumEquality` (`self.PlayerCombatState`) "PCS_CombatReady")) (`self.bCanAttack`))
      (set `self.bIsAttacking` true)
      (`self.SetAttackType` "AT_LightAttack")
      (else
        (set `self.bIsAttacking` false :!label _label_2)
        (`self.SetAttackType` "AT_None"))))
  (:`Released`
    (goto _label_2)))

(event `InputAction|HeavyAttack`
  (params (Key :type "Key Structure"))
  ;[1 1 1] IsAttacking - True/False
  (:`Pressed`
    (bind _returnvalue (`self.IsCharacterExhausted`))
    (if (and (and (not _returnvalue) (`|EnumEquality` (`self.PlayerCombatState`) "PCS_CombatReady")) (`self.bCanAttack`))
      (set `self.bIsAttacking` true)
      (`self.SetAttackType` "AT_HeavyAttack")
      (else
        (set `self.bIsAttacking` false :!label _label_3)
        (`self.SetAttackType` "AT_None"))))
  (:`Released`
    (goto _label_3)))

(event `self.ReceiveBeginPlay`
  (bind _returnvalue (`GameplayStatics.GetPlayerCameraManager` 0))
  ;[0.7231 0 0] BeginPlay
  (`|ExecutionSequence`
    (:`then_0`
      (set `Actor.Tags` (`|MakeArray` "Player" :!type "Name") (`GameplayStatics.GetPlayerCharacter` 0))
      (bind _returnvalue_2 (`|CreateWidget` "/Game/Widgets/WBP_Collectables.WBP_Collectables_C"))
      (bind _output_get (set `self.CollectableWidgetRef` _returnvalue_2))
      (`UserWidget.AddToViewport` _output_get 0))
    (:`then_1`
      (set `PlayerCameraManager.ViewPitchMax` (`self.CameraPitchMax`) _returnvalue)
      (set `PlayerCameraManager.ViewPitchMin` (`self.CameraPitchMin`) _returnvalue))
    (:`then_2`
      (bind _asweapon_base (cast `WeaponBase` (`ChildActorComponent.ChildActor` (`self.EquippedWeapon`))))
      (`self.AttachWeaponToSocket` (`WeaponBase.SheathSocket` _asweapon_base)))))

(event `self.ReceiveTick`
  (params (DeltaSeconds :type "Float (single-precision)"))
  ;[1 1 1] Tick
  (`self.GetEquippedWeaponInfo`)
  (`self.IKLegsOnTick`)
  (`self.AddToInventoryTrace`)
  (`KismetSystemLibrary.PrintString` (`KismetSystemLibrary.GetObjectName` (`self.LookedAtActor`)) true false (struct :`G` 0.66 :`B` 1.0 :`A` 1.0) (`GameplayStatics.GetWorldDeltaSeconds`)))

(event `Key|Gamepad_DPad_Up`
  (params (Key :type "Key Structure"))
  (bind _spotlight (`self.SpotLight`))
  ;[1 1 1] Enable/Disable SpotLight
  (:`Pressed`
    (`/Engine/EditorBlueprintResources/StandardMacros.FlipFlop` :!label _label_4
      (:`A`
        (`SceneComponent.SetVisibility` _spotlight true false))
      (:`B`
        (`SceneComponent.SetVisibility` _spotlight false false)))))

(event `Key|L`
  (params (Key :type "Key Structure"))
  ;[1 1 1] Enable/Disable SpotLight
  (:`Pressed`
    (goto _label_4)))

(event `InputAction|FocusTarget`
  (params (Key :type "Key Structure"))
  ;[1 1 1] Toggle LookAt
  (:`Pressed`
    (`/Engine/EditorBlueprintResources/StandardMacros.FlipFlop`
      (:`A`
        (set `self.LookAt` true))
      (:`B`
        (set `self.LookAt` false)))))

(event `AddToInventoryTrace`
  (bind (_outhit _returnvalue) (`KismetSystemLibrary.LineTraceSingle` :`Start` (`SceneComponent.GetSocketLocation` (`self.Mesh`) "HeadSocket") :`End` (`SceneComponent.K2_GetComponentLocation` (`self.ItemPickupArrow`)) :`TraceChannel` "TraceTypeQuery4" :`DrawDebugType` "ForOneFrame"))
  (if _returnvalue
    (set `self.LookedAtActor` (`.HitActor` (`GameplayStatics.BreakHitResult` _outhit)))
    (else
      (set `self.LookedAtActor` null))))

(event `ItemCollected_1`
  ;[1 1 1] Event - Item Collected
  (`/Game/Widgets/WBP_Collectables.UpdateText` (`self.CollectableWidgetRef`) (`KismetTextLibrary.Conv_IntToText` (`self.ItemsCollected`))))

(event `self.DoorOpenInteractionStarted`
  (params (InteractableActor :type "Actor Object Reference"))
  ;[1 1 1] DoorOpenInteractionStarted
  (if (not (`self.bIsInUninterruptableAction`))
    (`|PlayMontage` (`self.Mesh`) "/Game/Animations/Montages/Characters/M_DoorInteraction.M_DoorInteraction"
      (:`then`
        (set `self.bIsInUninterruptableAction` true)
        (`self.SetPlayerActionState` "PAS_Interacting")
        (bind _asinteractable_door (cast `InteractableDoor` InteractableActor))
        (`ActorComponent.Deactivate` (`self.CharacterMovement`)))
      (:`OnCompleted`
        (set `self.bIsInUninterruptableAction` false)
        (`self.SetPlayerActionState` "PAS_Idle")
        (`ActorComponent.Activate` (`self.CharacterMovement`) false))
      (:`OnNotifyBegin`
        (`InteractableDoor.OpenDoor` _asinteractable_door)))))

(event `InputAction|PickupItem`
  (params (Key :type "Key Structure"))
  (bind _lookedatactor (`self.LookedAtActor`))
  (:`Pressed`
    (`/Engine/EditorBlueprintResources/StandardMacros.IsValid` _lookedatactor
      (:`Is Valid`
        (`InventoryComponent.AddItemToInventory` (`self.InventoryComponent`) _lookedatactor -1))
      (:`Is Not Valid`
        (`KismetSystemLibrary.PrintString` "LookedAtActor is not valid")))))

(event `InputAction|Dodge` :consume false
  (params (Key :type "Key Structure"))
  (bind _pc (`self.PC`))
  ;[1 1 1] Dodge Roll Prototype
  (:`Pressed`
    (`/Engine/EditorBlueprintResources/StandardMacros.IsValid` _pc
      (:`Is Valid`
        (if (not (`RPGProjectPlayerController.bIsInMenu` _pc))
          (if (and (not (`self.bIsInUninterruptableAction`)) (not (`NavMovementComponent.IsFalling` (`self.CharacterMovement`))))
            (`|ExecutionSequence`
              (:`then_0`
                (`/Engine/EditorBlueprintResources/StandardMacros.DoOnce` false :!label _label_5
                  (:`Completed`
                    (`self.SetPlayerActionState` "PAS_Dodging")
                    (set `self.bIsInUninterruptableAction` true)
                    (set `self.bCanAttack` false)
                    (`|PlayMontage` (`self.Mesh`) "/Game/Animations/Montages/Characters/M_DodgeRoll.M_DodgeRoll" 1.0 0.0 (`self.DiveRollName`)
                      (:`OnCompleted`
                        (`self.SetPlayerActionState` "PAS_Idle"))
                      (:`OnBlendOut`
                        (set `self.bCanAttack` true)
                        (set `self.bIsInUninterruptableAction` false)
                        (goto _label_5 :!via `Reset`)))))))))))))

(event `Key|Nine`
  (params (Key :type "Key Structure"))
  (:`Pressed`
    (`InventoryComponent.SwapItems` (`self.InventoryComponent`) 0 1)))

(fn `AttachWeaponToSocket`
  (params (SocketName :type Name))
  (if (`SceneComponent.DoesSocketExist` (`self.Mesh`) SocketName)
    (bind _returnvalue (`SceneComponent.K2_AttachToComponent` (`Actor.RootComponent` (`ChildActorComponent.ChildActor` (`self.EquippedWeapon`))) (`self.Mesh`) SocketName "SnapToTarget" "SnapToTarget" "SnapToTarget" true))
    (else
      (`KismetSystemLibrary.PrintString` (`KismetStringLibrary.BuildString_Name` "Socket Name: " "" SocketName "doesn't exist")))))

(fn `GetEquippedWeaponInfo`
  (bind _equippedweapon (`self.EquippedWeapon`))
  (`/Engine/EditorBlueprintResources/StandardMacros.IsValid` _equippedweapon
    (:`Is Valid`
      (bind _asweapon_base (cast `WeaponBase` (`ChildActorComponent.ChildActor` _equippedweapon)))
      (set `self.EquippedWeaponCast` _asweapon_base)
      (`|ExecutionSequence`
        (:`then_0`
          (bind _weapontype (break `WeaponInfo` (`WeaponBase.WeaponInfo` _asweapon_base)))
          (`self.SetEquippedWeaponType` _weapontype)
          (switch `EWeaponType` _weapontype
            (:`WT_Unarmed`
              (set `self.DiveRollName` "UnarmedDiveRoll"))
            (:`WT_1HandSword`
              (set `self.DiveRollName` "ArmedDiveRoll"))
            (:`WT_2HandSpear`
              (set `self.DiveRollName` "2HandSpearDiveRoll"))))))))

(fn `IKFootTrace`
  (params (SocketName :type Name) (Distance :type "Float (double-precision)"))
  (returns (Location :type "Vector Structure") (FootTraceOffset :type "Float (double-precision)"))
  (bind (_returnvalue_x _returnvalue_y _returnvalue_z) (`KismetMathLibrary.BreakVector` (`self.K2_GetActorLocation`)))
  (bind (_returnvalue_x_2 _returnvalue_y_2 _returnvalue_z_2) (`KismetMathLibrary.BreakVector` (`SceneComponent.GetSocketLocation` (`self.Mesh`) SocketName)))
  (bind _result (`/Engine/EditorBlueprintResources/StandardMacros.NegateFloat` Distance)
    (:`  `
      (bind (_outhit _returnvalue) (`KismetSystemLibrary.LineTraceSingle` (`KismetMathLibrary.MakeVector` _returnvalue_x_2 _returnvalue_y_2 _returnvalue_z) (`KismetMathLibrary.MakeVector` _returnvalue_x_2 _returnvalue_y_2 (+ _returnvalue_z_2 _result)) "TraceTypeQuery3"))
      (if _returnvalue
        (bind (_bblockinghit _binitialoverlap _time _distance _location) (`GameplayStatics.BreakHitResult` _outhit))
        (bind (_returnvalue_x_3 _returnvalue_y_3 _returnvalue_z_3) (`KismetMathLibrary.BreakVector` (- _location (`SceneComponent.K2_GetComponentLocation` (`self.Mesh`)))))
        (return _location (- _returnvalue_z_3 (`self.IKHipOffset`)))
        (else
          (return (0.0 0.0 0.0) 0.0))))))

(fn `IKLegsOnTick`
  (bind _returnvalue (`GameplayStatics.GetWorldDeltaSeconds`))
  (`|ExecutionSequence`
    (:`then_0`
      (bind (_location _foottraceoffset) (`self.IKFootTrace` "foot_lSocket" (/ (`CapsuleComponent.CapsuleHalfHeight` (`self.CapsuleComponent`)) 1.5)))
      (set `self.IKLeftFootOffset` (`KismetMathLibrary.FInterpTo` (`self.IKLeftFootOffset`) _foottraceoffset (`GameplayStatics.GetWorldDeltaSeconds`) 20.0)))
    (:`then_1`
      (bind (_location_2 _foottraceoffset_2) (`self.IKFootTrace` "foot_rSocket" (/ (`CapsuleComponent.CapsuleHalfHeight` (`self.CapsuleComponent`)) 1.5)))
      (set `self.IKRightFootOffset` (`KismetMathLibrary.FInterpTo` (`self.IKRightFootOffset`) _foottraceoffset_2 _returnvalue 20.0))
      (bind (_returnvalue_x _returnvalue_y _returnvalue_z) (`KismetMathLibrary.BreakVector` (- _location _location_2)))
      (bind _returnvalue_2 (`KismetMathLibrary.Abs` _returnvalue_z))
      (set `self.IKHipOffset` (`KismetMathLibrary.FInterpTo` (`self.IKHipOffset`) (`KismetMathLibrary.SelectFloat` (* _returnvalue_2 -0.5) 0.0 (< _returnvalue_2 50.0)) _returnvalue 20.0)))))

(fn `SetRotationToInput`
  (bind _asbp_rpgproject_player_controller (cast `/Game/Characters/Player/BP_RPGProjectPlayerController` (`GameplayStatics.GetPlayerController` 0)))
  (if (and (!= (`RPGProjectPlayerController.ForwardValue` _asbp_rpgproject_player_controller) 0.0) (!= (`RPGProjectPlayerController.RightValue` _asbp_rpgproject_player_controller) 0.0))
    (`self.K2_SetActorRotation` (`RPGProjectPlayerController.PlayerInputRotation` _asbp_rpgproject_player_controller))))

(fn `UserConstructionScript`)